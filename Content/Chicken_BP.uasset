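; Chicken_BP is an input-driven chicken pawn with simple hand-rolled movement.
; MoveForward and MoveRight axis events add movement input along the actor's forward and right vectors, scaled by MaxSpeed.
; Tick consumes that input and applies it, scaled by delta time, as a swept AddActorLocalOffset, so world-space directions are treated as local ones.
; BeginPlay, overlap and construction logic are empty.
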(event EventBeginPlay)

(event Collision|EventActorBeginOverlap
  (params (OtherActor :type Actor%20Object%20Reference)))

(event EventTick
  (params (DeltaSeconds :type Float%20%28single-precision%29))
  (bind _returnvalue (Class|Pawn|ConsumeMovementInputVector))
  (Transformation|AddActorLocalOffset (* _returnvalue DeltaSeconds) true false))

(event Input|AxisEvents|InputAxisMoveForward
  (params (AxisValue :type Float%20%28single-precision%29))
  (Pawn|Input|AddMovementInput (Transformation|GetActorForwardVector) (* AxisValue (Variables|Default|GetMaxSpeed)) false))

(event Input|AxisEvents|InputAxisMoveRight
  (params (AxisValue :type Float%20%28single-precision%29))
  (Pawn|Input|AddMovementInput (Transformation|GetActorRightVector) (* (Variables|Default|GetMaxSpeed) AxisValue) false))

(fn ConstructionScript)