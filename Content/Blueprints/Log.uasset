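; Log actor that moves along world Y at its ForwardSpeed, with a chance of carrying a coin.
; On BeginPlay, Randomize picks a short, medium or tall variant, setting Size, mesh and matching material, and fixes the rotation.
; After a brief delay, SpawnCoin occasionally spawns a Coin above the log and copies ForwardSpeed to it so both move at the same speed.
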(event EventBeginPlay
  (CallFunction|Randomize)
  (Utilities|FlowControl|Delay 0.2)
  (CallFunction|SpawnCoin))

(event Collision|EventActorBeginOverlap
  (params (OtherActor :type Actor%20Object%20Reference)))

(event EventTick
  (params (DeltaSeconds :type Float%20%28single-precision%29))
  (Transformation|AddActorWorldOffset (Math|Vector|MakeVector 0.0 (* DeltaSeconds (Variables|Default|GetForwardSpeed)) 0.0)))

(fn ConstructionScript)

(fn Randomize
  (bind _output_get (LocalVariables|SetRandomInt (Math|Random|RandomIntegerinRange 0 2)))
  (Variables|Default|SetSize _output_get)
  (Components|StaticMesh|SetStaticMesh (Variables|Default|GetStaticMesh) (Utilities|Select :Index _output_get :Option%200 "/Game/Meshes/Log_Short_Mesh.Log_Short_Mesh" :Option%201 "/Game/Meshes/Log_Medium_Mesh.Log_Medium_Mesh" :Option%202 "/Game/Meshes/Log_Tall_Mesh.Log_Tall_Mesh"))
  (Rendering|Material|SetMaterial (Variables|Default|GetStaticMesh) 0 (Utilities|Select :Index _output_get :Option%200 "/Game/Materials/Log_Short_Material.Log_Short_Material" :Option%201 "/Game/Materials/Log_Medium_Material.Log_Medium_Material" :Option%202 "/Game/Materials/Log_Tall_Material.Log_Tall_Material"))
  (Transformation|SetActorRotation "0,90.000000, 0"))

(fn SpawnCoin
  (if (Math|Random|RandomBoolwithWeight 0.1)
    (bind _returnvalue (Game|SpawnActorfromClass "/Game/Blueprints/Coin.Coin_C" (Math|Transform|MakeTransform (+ (Transformation|GetActorLocation) "0, 0,55.000000") "0,90.000000, 0" "1,1,1") "Undefined" 0 0))
    (Variables|/Game/Blueprints/Coin.Coin_C|SetForwardSpeed _returnvalue (Variables|Default|GetForwardSpeed))))