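; Train is a moving train car hazard that kills the Chicken on contact.
; Shortly after BeginPlay, Randomize picks the back, middle or front mesh and material from the Type variable, despite its name using no randomness.
; Tick moves the actor along world Y at ForwardSpeed, scaled by delta time.
; A Box overlap casts the other actor to Chicken and sets IsDead.
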(event OnComponentBeginOverlap(Box)
  (params (OverlappedComponent :type Primitive%20Component%20Object%20Reference) (OtherActor :type Actor%20Object%20Reference) (OtherComp :type Primitive%20Component%20Object%20Reference) (OtherBodyIndex :type Integer) (bFromSweep :type Boolean) (SweepResult :type Hit%20Result%20Structure%20%28by%20ref%29))
  (bind _aschicken (Utilities|Casting|CastToChicken OtherActor))
  (Variables|/Game/Blueprints/Chicken.Chicken_C|SetIsDead _aschicken true))

(event EventBeginPlay
  (Utilities|FlowControl|Delay 0.2)
  (CallFunction|Randomize))

(event Collision|EventActorBeginOverlap
  (params (OtherActor :type Actor%20Object%20Reference)))

(event EventTick
  (params (DeltaSeconds :type Float%20%28single-precision%29))
  (Transformation|AddActorWorldOffset (Math|Vector|MakeVector 0.0 (* DeltaSeconds (Variables|Default|GetForwardSpeed)) 0.0)))

(fn ConstructionScript)

(fn Randomize
  (bind _staticmesh (Variables|Default|GetStaticMesh))
  (bind _staticmesh_2 (Variables|Default|GetStaticMesh))
  (switch int (Variables|Default|GetType)
    (:0
      (Components|StaticMesh|SetStaticMesh _staticmesh "/Game/Meshes/Train_Back_Mesh.Train_Back_Mesh")
      (Rendering|Material|SetMaterial _staticmesh_2 0 "/Game/Materials/Train_Back_Material.Train_Back_Material"))
    (:1
      (Components|StaticMesh|SetStaticMesh _staticmesh "/Game/Meshes/Train_Middle_Mesh.Train_Middle_Mesh")
      (Rendering|Material|SetMaterial _staticmesh_2 0 "/Game/Materials/Train_Middle_Material.Train_Middle_Material"))
    (:2
      (Components|StaticMesh|SetStaticMesh _staticmesh "/Game/Meshes/Train_Front_Mesh.Train_Front_Mesh")
      (Rendering|Material|SetMaterial _staticmesh_2 0 "/Game/Materials/Train_Front_Material.Train_Front_Material"))))