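; Obstacle actor that randomly becomes a bush, a short, medium or tall tree, or one of two rocks.
; On BeginPlay, Randomize rolls one integer that selects both the static mesh and its matching material, keeping the pair in sync.
; Rock variants then get a second roll that sets the actor's rotation to a random quarter-turn step, while vegetation keeps its existing rotation.
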(event EventBeginPlay
  (CallFunction|Randomize))

(event Collision|EventActorBeginOverlap
  (params (OtherActor :type Actor%20Object%20Reference)))

(event EventTick
  (params (DeltaSeconds :type Float%20%28single-precision%29)))

(fn ConstructionScript)

(fn Randomize
  (bind _output_get (LocalVariables|SetRandomInt (Math|Random|RandomIntegerinRange 0 5)))
  (Components|StaticMesh|SetStaticMesh (Variables|Default|GetStaticMesh) (Utilities|Select :Index _output_get :Option%200 "/Game/Meshes/Bush_Mesh.Bush_Mesh" :Option%201 "/Game/Meshes/Tree_Short_Mesh.Tree_Short_Mesh" :Option%202 "/Game/Meshes/Tree_Medium_Mesh.Tree_Medium_Mesh" :Option%203 "/Game/Meshes/Tree_Tall_Mesh.Tree_Tall_Mesh" :Option%204 "/Game/Meshes/Rock_V1_Mesh.Rock_V1_Mesh" :Option%205 "/Game/Meshes/Rock_V2_Mesh.Rock_V2_Mesh"))
  (Rendering|Material|SetMaterial (Variables|Default|GetStaticMesh) 0 (Utilities|Select :Index _output_get :Option%200 "/Game/Materials/Bush_Material.Bush_Material" :Option%201 "/Game/Materials/Tree_Short_Material.Tree_Short_Material" :Option%202 "/Game/Materials/Tree_Medium_Material.Tree_Medium_Material" :Option%203 "/Game/Materials/Tree_Tall_Material.Tree_Tall_Material" :Option%204 "/Game/Materials/Rock_V1_Material.Rock_V1_Material" :Option%205 "/Game/Materials/Rock_V2_Material.Rock_V2_Material"))
  (if (>= _output_get 4)
    (switch int (Math|Random|RandomIntegerinRange 0 3)
      (:0
        (Transformation|SetActorRotation "0, 0, 0"))
      (:1
        (Transformation|SetActorRotation "0,90.000000, 0"))
      (:2
        (Transformation|SetActorRotation "0,180.000000, 0"))
      (:3
        (Transformation|SetActorRotation "0,270.000000, 0")))))