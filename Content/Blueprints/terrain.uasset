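; Grass terrain strip that scatters obstacles and coins for the Chicken and kills it at the side borders.
; On BeginPlay, Randomize applies the grass material, lowers and rotates the actor, then makes one or two random picks among nine evenly spaced slots.
; A DoOnce per slot prevents double spawns; each spawns an Obstacle or occasionally a Coin, likelier toward the centre.
; Overlapping either border sets the Chicken's IsDead.
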(event OnComponentBeginOverlap(LChickenBorder)
  (params (OverlappedComponent :type Primitive%20Component%20Object%20Reference) (OtherActor :type Actor%20Object%20Reference) (OtherComp :type Primitive%20Component%20Object%20Reference) (OtherBodyIndex :type Integer) (bFromSweep :type Boolean) (SweepResult :type Hit%20Result%20Structure%20%28by%20ref%29))
  (bind _aschicken (Utilities|Casting|CastToChicken OtherActor))
  (Variables|/Game/Blueprints/Chicken.Chicken_C|SetIsDead _aschicken true))

(event OnComponentBeginOverlap(RChickenBorder)
  (params (OverlappedComponent :type Primitive%20Component%20Object%20Reference) (OtherActor :type Actor%20Object%20Reference) (OtherComp :type Primitive%20Component%20Object%20Reference) (OtherBodyIndex :type Integer) (bFromSweep :type Boolean) (SweepResult :type Hit%20Result%20Structure%20%28by%20ref%29))
  (bind _aschicken (Utilities|Casting|CastToChicken OtherActor))
  (Variables|/Game/Blueprints/Chicken.Chicken_C|SetIsDead _aschicken true))

(event EventBeginPlay
  (CallFunction|Randomize))

(event Collision|EventActorBeginOverlap
  (params (OtherActor :type Actor%20Object%20Reference)))

(event EventTick
  (params (DeltaSeconds :type Float%20%28single-precision%29)))

(fn ConstructionScript)

(fn Randomize
  (bind _returnvalue (Transformation|GetActorTransform))
  (bind _returnvalue_2 (+ (.location _returnvalue) "0,-300.000000,40.000000"))
  (bind _returnvalue_3 (+ (.location _returnvalue) "0,-400.000000,40.000000"))
  (bind _returnvalue_4 (+ (.location _returnvalue) "0, 0,40.000000"))
  (bind _returnvalue_5 (+ (.location _returnvalue) "0,100.000000,40.000000"))
  (bind _returnvalue_6 (+ (.location _returnvalue) "0,200.000000,40.000000"))
  (bind _returnvalue_7 (+ (.location _returnvalue) "0,300.000000,40.000000"))
  (bind _returnvalue_8 (+ (.location _returnvalue) "0,400.000000,40.000000"))
  (bind _returnvalue_9 (+ (.location _returnvalue) "0,-100.000000,40.000000"))
  (bind _returnvalue_10 (+ (.location _returnvalue) "0,-200.000000,40.000000"))
  (Rendering|Material|SetMaterial (Variables|Default|GetStaticMesh) 0 "/Game/Materials/Grass_Material.Grass_Material")
  (Transformation|SetActorLocationAndRotation (+ (Transformation|GetActorLocation) "0, 0,-45.000000") "0,90.000000, 0")
  (bind _output_get (LocalVariables|SetObstacleNumber (Math|Random|RandomIntegerinRange 0 1)))
  (for _index (range 0 _output_get)
    (switch int (Math|Random|RandomIntegerinRange 0 8)
      (:0
        (Utilities|FlowControl|DoOnce false
          (:Completed
            (if (Math|Random|RandomBoolwithWeight 0.05)
              (Game|SpawnActorfromClass "/Game/Blueprints/Coin.Coin_C" (Math|Transform|MakeTransform (+ _returnvalue_8 "0, 0,10.000000") "0,90.000000, 0" "1,1,1") "Undefined" 0 0)
              (else
                (Game|SpawnActorfromClass "/Game/Blueprints/Obstacle.Obstacle_C" (Math|Transform|MakeTransform _returnvalue_8 "0, 0, 0" "1,1,1") "Undefined" 0 0))))))
      (:1
        (Utilities|FlowControl|DoOnce false
          (:Completed
            (if (Math|Random|RandomBoolwithWeight 0.05)
              (Game|SpawnActorfromClass "/Game/Blueprints/Coin.Coin_C" (Math|Transform|MakeTransform (+ _returnvalue_7 "0, 0,10.000000") "0,90.000000, 0" "1,1,1") "Undefined" 0 0)
              (else
                (Game|SpawnActorfromClass "/Game/Blueprints/Obstacle.Obstacle_C" (Math|Transform|MakeTransform _returnvalue_7 "0, 0, 0" "1,1,1") "Undefined" 0 0))))))
      (:2
        (Utilities|FlowControl|DoOnce false
          (:Completed
            (if (Math|Random|RandomBoolwithWeight 0.1)
              (Game|SpawnActorfromClass "/Game/Blueprints/Coin.Coin_C" (Math|Transform|MakeTransform (+ _returnvalue_6 "0, 0,10.000000") "0,90.000000, 0" "1,1,1") "Undefined" 0 0)
              (else
                (Game|SpawnActorfromClass "/Game/Blueprints/Obstacle.Obstacle_C" (Math|Transform|MakeTransform _returnvalue_6 "0, 0, 0" "1,1,1") "Undefined" 0 0))))))
      (:3
        (Utilities|FlowControl|DoOnce false
          (:Completed
            (if (Math|Random|RandomBoolwithWeight 0.1)
              (Game|SpawnActorfromClass "/Game/Blueprints/Coin.Coin_C" (Math|Transform|MakeTransform (+ _returnvalue_5 "0, 0,10.000000") "0,90.000000, 0" "1,1,1") "Undefined" 0 0)
              (else
                (Game|SpawnActorfromClass "/Game/Blueprints/Obstacle.Obstacle_C" (Math|Transform|MakeTransform _returnvalue_5 "0, 0, 0" "1,1,1") "Undefined" 0 0))))))
      (:4
        (Utilities|FlowControl|DoOnce false
          (:Completed
            (if (Math|Random|RandomBoolwithWeight 0.2)
              (Game|SpawnActorfromClass "/Game/Blueprints/Coin.Coin_C" (Math|Transform|MakeTransform (+ _returnvalue_4 "0, 0,10.000000") "0,90.000000, 0" "1,1,1") "Undefined" 0 0)
              (else
                (Game|SpawnActorfromClass "/Game/Blueprints/Obstacle.Obstacle_C" (Math|Transform|MakeTransform _returnvalue_4 "0, 0, 0" "1,1,1") "Undefined" 0 0))))))
      (:5
        (Utilities|FlowControl|DoOnce false
          (:Completed
            (if (Math|Random|RandomBoolwithWeight 0.1)
              (Game|SpawnActorfromClass "/Game/Blueprints/Coin.Coin_C" (Math|Transform|MakeTransform (+ _returnvalue_9 "0, 0,10.000000") "0,90.000000, 0" "1,1,1") "Undefined" 0 0)
              (else
                (Game|SpawnActorfromClass "/Game/Blueprints/Obstacle.Obstacle_C" (Math|Transform|MakeTransform _returnvalue_9 "0, 0, 0" "1,1,1") "Undefined" 0 0))))))
      (:6
        (Utilities|FlowControl|DoOnce false
          (:Completed
            (if (Math|Random|RandomBoolwithWeight 0.1)
              (Game|SpawnActorfromClass "/Game/Blueprints/Coin.Coin_C" (Math|Transform|MakeTransform (+ _returnvalue_10 "0, 0,10.000000") "0,90.000000, 0" "1,1,1") "Undefined" 0 0)
              (else
                (Game|SpawnActorfromClass "/Game/Blueprints/Obstacle.Obstacle_C" (Math|Transform|MakeTransform _returnvalue_10 "0, 0, 0" "1,1,1") "Undefined" 0 0))))))
      (:7
        (Utilities|FlowControl|DoOnce false
          (:Completed
            (if (Math|Random|RandomBoolwithWeight 0.05)
              (Game|SpawnActorfromClass "/Game/Blueprints/Coin.Coin_C" (Math|Transform|MakeTransform (+ _returnvalue_2 "0, 0,10.000000") "0,90.000000, 0" "1,1,1") "Undefined" 0 0)
              (else
                (Game|SpawnActorfromClass "/Game/Blueprints/Obstacle.Obstacle_C" (Math|Transform|MakeTransform _returnvalue_2 "0, 0, 0" "1,1,1") "Undefined" 0 0))))))
      (:8
        (Utilities|FlowControl|DoOnce false
          (:Completed
            (if (Math|Random|RandomBoolwithWeight 0.05)
              (Game|SpawnActorfromClass "/Game/Blueprints/Coin.Coin_C" (Math|Transform|MakeTransform (+ _returnvalue_3 "0, 0,10.000000") "0,90.000000, 0" "1,1,1") "Undefined" 0 0)
              (else
                (Game|SpawnActorfromClass "/Game/Blueprints/Obstacle.Obstacle_C" (Math|Transform|MakeTransform _returnvalue_3 "0, 0, 0" "1,1,1") "Undefined" 0 0)))))))))