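; Road lane actor for a chicken-crossing game that spawns cars or trucks driving across it.
; On BeginPlay it picks direction and material from its X position, so lanes can alternate, then randomly chooses a mostly-car vehicle type.
; After a random start delay it spawns that first vehicle, then five more of the same type at random intervals.
; Border volumes destroy vehicles leaving them and kill any chicken that enters.
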(event OnComponentEndOverlap(LeftBorder)
  (params (OverlappedComponent :type Primitive%20Component%20Object%20Reference) (OtherActor :type Actor%20Object%20Reference) (OtherComp :type Primitive%20Component%20Object%20Reference) (OtherBodyIndex :type Integer))
  (Utilities|FlowControl|Sequence
    (:then_0
      (bind _ascar (Utilities|Casting|CastToCar OtherActor))
      (Actor|DestroyActor _ascar))
    (:then_1
      (bind _astruck (Utilities|Casting|CastToTruck OtherActor))
      (Actor|DestroyActor _astruck))))

(event OnComponentEndOverlap(RightBorder)
  (params (OverlappedComponent :type Primitive%20Component%20Object%20Reference) (OtherActor :type Actor%20Object%20Reference) (OtherComp :type Primitive%20Component%20Object%20Reference) (OtherBodyIndex :type Integer))
  (Utilities|FlowControl|Sequence
    (:then_0
      (bind _ascar (Utilities|Casting|CastToCar OtherActor))
      (Actor|DestroyActor _ascar))
    (:then_1
      (bind _astruck (Utilities|Casting|CastToTruck OtherActor))
      (Actor|DestroyActor _astruck))))

(event OnComponentBeginOverlap(LeftBorder)
  (params (OverlappedComponent :type Primitive%20Component%20Object%20Reference) (OtherActor :type Actor%20Object%20Reference) (OtherComp :type Primitive%20Component%20Object%20Reference) (OtherBodyIndex :type Integer) (bFromSweep :type Boolean) (SweepResult :type Hit%20Result%20Structure%20%28by%20ref%29))
  (bind _aschicken_bp (Utilities|Casting|CastToChicken_BP OtherActor))
  (Variables|/Game/Blueprints/Chicken_BP.Chicken_BP_C|SetIsDead _aschicken_bp true))

(event OnComponentBeginOverlap(RightBorder)
  (params (OverlappedComponent :type Primitive%20Component%20Object%20Reference) (OtherActor :type Actor%20Object%20Reference) (OtherComp :type Primitive%20Component%20Object%20Reference) (OtherBodyIndex :type Integer) (bFromSweep :type Boolean) (SweepResult :type Hit%20Result%20Structure%20%28by%20ref%29))
  (bind _aschicken_bp (Utilities|Casting|CastToChicken_BP OtherActor))
  (Variables|/Game/Blueprints/Chicken_BP.Chicken_BP_C|SetIsDead _aschicken_bp true))

(event EventBeginPlay
  (CallFunction|DetermineDirection)
  (Utilities|FlowControl|Delay (Math|Random|RandomFloatinRange 0.0 5.0))
  (CallFunction|SpawnVehicle)
  (Utilities|FlowControl|Delay (Math|Random|RandomFloatinRange 5.0 7.0))
  (CallFunction|SpawnAnother)
  (Utilities|FlowControl|Delay (Math|Random|RandomFloatinRange 5.0 7.0))
  (CallFunction|SpawnAnother)
  (Utilities|FlowControl|Delay (Math|Random|RandomFloatinRange 5.0 7.0))
  (CallFunction|SpawnAnother)
  (Utilities|FlowControl|Delay (Math|Random|RandomFloatinRange 5.0 7.0))
  (CallFunction|SpawnAnother)
  (Utilities|FlowControl|Delay (Math|Random|RandomFloatinRange 5.0 7.0))
  (CallFunction|SpawnAnother))

(event Collision|EventActorBeginOverlap
  (params (OtherActor :type Actor%20Object%20Reference)))

(event EventTick
  (params (DeltaSeconds :type Float%20%28single-precision%29)))

(fn ConstructionScript)

(fn DetermineDirection
  (Components|StaticMesh|SetStaticMesh (Variables|Default|GetStaticMesh) "/Game/Meshes/Road_Mesh.Road_Mesh")
  (if (== (Math|Float|%(Float) (.x (Transformation|GetActorLocation)) 2e+02) 0.0)
    (Rendering|Material|SetMaterial (Variables|Default|GetStaticMesh) 0 "/Game/Materials/Road_Stripes_Material.Road_Stripes_Material")
    (Variables|Default|SetDirectionToRight true)
    (else
      (Rendering|Material|SetMaterial (Variables|Default|GetStaticMesh) 0 "/Game/Materials/Road_Material.Road_Material")
      (Variables|Default|SetDirectionToRight false)))
  (Transformation|SetActorRotation "0,90.000000, 0"))

(fn SpawnVehicle
  (bind _returnvalue (Transformation|GetActorTransform))
  (bind _returnvalue_2 (Math|Random|RandomBoolwithWeight 0.85))
  (bind _returnvalue_3 (+ (.location _returnvalue) "0.000000,-1000.000000,25.000000"))
  (bind _returnvalue_4 (+ (.location _returnvalue) "0,1000.000000,25.000000"))
  (if (Variables|Default|GetDirectionToRight)
    (if _returnvalue_2
      (bind _returnvalue_5 (Game|SpawnActorfromClass "/Game/Blueprints/Car.Car_C" (Math|Transform|MakeTransform _returnvalue_3 "0, 0, 0" "1,1,1") "Undefined" 0 0))
      (Variables|/Game/Blueprints/Car.Car_C|SetForwardSpeed _returnvalue_5 2e+02)
      (Variables|Default|SetVehicleIsCar true :!label _label)
      (else
        (bind _returnvalue_6 (Game|SpawnActorfromClass "/Game/Blueprints/Truck.Truck_C" (Math|Transform|MakeTransform _returnvalue_3 "0, 0, 0" "1,1,1") "Undefined" 0 0))
        (Variables|/Game/Blueprints/Truck.Truck_C|SetForwardSpeed _returnvalue_6 3e+02)
        (Variables|Default|SetVehicleIsCar false :!label _label_2)))
    (elif _returnvalue_2
      (bind _returnvalue_7 (Game|SpawnActorfromClass "/Game/Blueprints/Car.Car_C" (Math|Transform|MakeTransform _returnvalue_4 "0,180.000000, 0" "1,1,1") "Undefined" 0 0))
      (Variables|/Game/Blueprints/Car.Car_C|SetForwardSpeed _returnvalue_7 -2e+02)
      (goto _label)
      (else
        (bind _returnvalue_8 (Game|SpawnActorfromClass "/Game/Blueprints/Truck.Truck_C" (Math|Transform|MakeTransform _returnvalue_4 "0,180.000000, 0" "1,1,1") "Undefined" 0 0))
        (Variables|/Game/Blueprints/Truck.Truck_C|SetForwardSpeed _returnvalue_8 -3e+02)
        (goto _label_2)))))

(fn SpawnAnother
  (bind _returnvalue (Transformation|GetActorTransform))
  (bind _returnvalue_2 (+ (.location _returnvalue) "0.000000,-1000.000000,25.000000"))
  (bind _returnvalue_3 (+ (.location _returnvalue) "0,1000.000000,25.000000"))
  (if (Variables|Default|GetVehicleIsCar)
    (if (Variables|Default|GetDirectionToRight)
      (bind _returnvalue_4 (Game|SpawnActorfromClass "/Game/Blueprints/Car.Car_C" (Math|Transform|MakeTransform _returnvalue_2 "0, 0, 0" "1,1,1") "Undefined" 0 0))
      (Variables|/Game/Blueprints/Car.Car_C|SetForwardSpeed _returnvalue_4 2e+02)
      (else
        (bind _returnvalue_5 (Game|SpawnActorfromClass "/Game/Blueprints/Car.Car_C" (Math|Transform|MakeTransform _returnvalue_3 "0,180.000000, 0" "1,1,1") "Undefined" 0 0))
        (Variables|/Game/Blueprints/Car.Car_C|SetForwardSpeed _returnvalue_5 -2e+02)))
    (elif (Variables|Default|GetDirectionToRight)
      (bind _returnvalue_6 (Game|SpawnActorfromClass "/Game/Blueprints/Truck.Truck_C" (Math|Transform|MakeTransform _returnvalue_2 "0, 0, 0" "1,1,1") "Undefined" 0 0))
      (Variables|/Game/Blueprints/Truck.Truck_C|SetForwardSpeed _returnvalue_6 3e+02)
      (else
        (bind _returnvalue_7 (Game|SpawnActorfromClass "/Game/Blueprints/Truck.Truck_C" (Math|Transform|MakeTransform _returnvalue_3 "0,180.000000, 0" "1,1,1") "Undefined" 0 0))
        (Variables|/Game/Blueprints/Truck.Truck_C|SetForwardSpeed _returnvalue_7 -3e+02)))))