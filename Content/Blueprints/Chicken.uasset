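; Chicken is a player-controlled character that hops in fixed steps in four directions, apparently in a Crossy Road-style game.
; Each hop input jumps, offsets the static mesh and resets an idle timer, while the A key turns the actor.
; Tick calls EagleSpawn to spawn an actor near the chicken after prolonged idling, or flattens it and plays a sound once when IsDead.
; BeginPlay creates the HUD widget.
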(event EventBeginPlay
  (bind _returnvalue (UserInterface|CreateWidget "/Game/UI/WBP_HUD.WBP_HUD_C"))
  (bind _output_get (Variables|Default|SetWBP_HUD _returnvalue))
  (UserInterface|Viewport|AddtoViewport _output_get 0))

(event Collision|EventActorBeginOverlap
  (params (OtherActor :type Actor%20Object%20Reference)))

(event EventTick
  (params (DeltaSeconds :type Float%20%28single-precision%29))
  (bind _output_get (Variables|Default|SetIdleTime (+ DeltaSeconds (Variables|Default|GetIdleTime))))
  (if (>= _output_get 5.0)
    (Variables|Default|SetLocation (.location (Transformation|GetActorTransform)))
    (CallFunction|EagleSpawn)
    (Variables|Default|SetIdleTime 0.0)
    (elif (Variables|Default|GetIsDead)
      (Transformation|SetActorScale3D "1.000000,1.000000,0.050000")
      (Utilities|FlowControl|DoOnce false
        (:Completed
          (Audio|PlaySoundatLocation "/Game/Audio/CHICKEN_Cue.CHICKEN_Cue" "0, 0, 0" "0, 0, 0" 1.0 1.0 0.0 0 0 0))))))

(event Input|ActionEvents|InputActionJumpForward
  (params (Key :type Key%20Structure :default "None"))
  (:Pressed
    (if (not (Variables|Default|GetIsDead))
      (Character|Jump)
      (Transformation|SetWorldLocation (Variables|Default|GetStaticMesh) (+ (Transformation|GetWorldLocation (Variables|Default|GetStaticMesh)) "-100.000000, 0, 0") false false)
      (Utilities|FlowControl|Delay 0.5)
      (Character|StopJumping)
      (Variables|Default|SetIdleTime 0.0))))

(event Input|ActionEvents|InputActionJumpBackward
  (params (Key :type Key%20Structure :default "None"))
  (:Pressed
    (if (not (Variables|Default|GetIsDead))
      (Character|Jump)
      (Transformation|SetWorldLocation (Variables|Default|GetStaticMesh) (+ (Transformation|GetWorldLocation (Variables|Default|GetStaticMesh)) "100.000000, 0, 0") false false)
      (Utilities|FlowControl|Delay 0.5)
      (Character|StopJumping)
      (Variables|Default|SetIdleTime 0.0))))

(event Input|ActionEvents|InputActionJumpRight
  (params (Key :type Key%20Structure :default "None"))
  (:Pressed
    (if (not (Variables|Default|GetIsDead))
      (Character|Jump)
      (Transformation|SetWorldLocation (Variables|Default|GetStaticMesh) (+ (Transformation|GetWorldLocation (Variables|Default|GetStaticMesh)) "0.000000,-100.000000, 0") false false)
      (Utilities|FlowControl|Delay 0.5)
      (Character|StopJumping)
      (Variables|Default|SetIdleTime 0.0))))

(event Input|ActionEvents|InputActionJumpLeft
  (params (Key :type Key%20Structure :default "None"))
  (:Pressed
    (if (not (Variables|Default|GetIsDead))
      (Character|Jump)
      (Transformation|SetWorldLocation (Variables|Default|GetStaticMesh) (+ (Transformation|GetWorldLocation (Variables|Default|GetStaticMesh)) "0.000000,100.000000, 0") false false)
      (Utilities|FlowControl|Delay 0.5)
      (Character|StopJumping)
      (Variables|Default|SetIdleTime 0.0))))

(event Input|KeyboardEvents|A
  (params (Key :type Key%20Structure :default "None"))
  (:Pressed
    (Utilities|FlowControl|DoOnce false :!label _label
      (:Completed
        (Transformation|SetActorRotation (Math|Rotator|MakeRotator 0.0 0.0 (+ (.yaw (Transformation|GetActorRotation)) -9e+01))))))
  (:Released
    (goto _label Reset)))

(fn ConstructionScript)

(fn EagleSpawn
  (Game|SpawnActorfromClass "/Game/Blueprints/Eagle.Eagle_C" (Math|Transform|MakeTransform (+ (Variables|Default|GetLocation) "-300.000000, 0, 0") "0, 0, 0" "1,1,1") "Undefined" 0 0))