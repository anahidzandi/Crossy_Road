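; Truck is an obstacle actor that drives forward and kills any Chicken it runs into.
; On BeginPlay, Randomize picks a blue or red truck mesh with matching material and sets the collision box extent.
; Tick moves the truck along world Y at ForwardSpeed, scaled by delta time.
; The Box's overlap event casts the other actor to Chicken and sets its IsDead flag.
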(event OnComponentBeginOverlap(Box)
  (params (OverlappedComponent :type Primitive%20Component%20Object%20Reference) (OtherActor :type Actor%20Object%20Reference) (OtherComp :type Primitive%20Component%20Object%20Reference) (OtherBodyIndex :type Integer) (bFromSweep :type Boolean) (SweepResult :type Hit%20Result%20Structure%20%28by%20ref%29))
  (bind _aschicken (Utilities|Casting|CastToChicken OtherActor))
  (Variables|/Game/Blueprints/Chicken.Chicken_C|SetIsDead _aschicken true))

(event EventBeginPlay
  (CallFunction|Randomize))

(event Collision|EventActorBeginOverlap
  (params (OtherActor :type Actor%20Object%20Reference)))

(event EventTick
  (params (DeltaSeconds :type Float%20%28single-precision%29))
  (Transformation|AddActorWorldOffset (Math|Vector|MakeVector 0.0 (* DeltaSeconds (Variables|Default|GetForwardSpeed)) 0.0)))

(fn ConstructionScript)

(fn Randomize
  (bind _output_get (LocalVariables|SetRandomInt (Math|Random|RandomIntegerinRange 0 1)))
  (Components|StaticMesh|SetStaticMesh (Variables|Default|GetStaticMesh) (Utilities|Select :Index _output_get :Option%200 "/Game/Meshes/Truck_Blue_Mesh.Truck_Blue_Mesh" :Option%201 "/Game/Meshes/Truck_Red_Mesh.Truck_Red_Mesh"))
  (Rendering|Material|SetMaterial (Variables|Default|GetStaticMesh) 0 (Utilities|Select :Index _output_get :Option%200 "/Game/Materials/Truck_Blue_Material.Truck_Blue_Material" :Option%201 "/Game/Materials/Truck_Red_Material.Truck_Red_Material"))
  (Components|Box|SetBoxExtent (Variables|Default|GetBox) (Utilities|Select :Index _output_get :Option%200 "55.000000,151.000000,32.000000" :Option%201 "55.000000,151.000000,32.000000") true))