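; Block spawner that builds a strip of terrain, river and railroad rows when play begins by calling SpawnBiome repeatedly.
; SpawnBiome alternates terrain with a randomly picked other biome and rolls a random length, with a longer range for the third random type.
; Each biome spawns row actors along negative X, advancing SpawnLocation and RowCount.
; The third random type's spawn has no class set.
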(event EventBeginPlay
  (CallFunction|SpawnBiome)
  (CallFunction|SpawnBiome)
  (CallFunction|SpawnBiome)
  (CallFunction|SpawnBiome)
  (CallFunction|SpawnBiome)
  (CallFunction|SpawnBiome)
  (CallFunction|SpawnBiome)
  (CallFunction|SpawnBiome)
  (CallFunction|SpawnBiome))

(event Collision|EventActorBeginOverlap
  (params (OtherActor :type Actor%20Object%20Reference)))

(event EventTick
  (params (DeltaSeconds :type Float%20%28single-precision%29)))

(fn ConstructionScript)

(fn SpawnBiome
  (if (== (Variables|Default|GetCurrentBiomeType) 0)
    (bind _output_get (Variables|Default|SetCurrentBiomeType (Math|Random|RandomIntegerinRange 1 3)))
    (else
      (Variables|Default|SetCurrentBiomeType 0)))
  (if (< _output_get 3)
    (Variables|Default|SetCurrentBiomeLength (Math|Random|RandomIntegerinRange 1 4))
    (else
      (Variables|Default|SetCurrentBiomeLength (Math|Random|RandomIntegerinRange 2 6))))
  (switch int (Variables|Default|GetCurrentBiomeType)
    (:0
      (for _index (range 0 (Variables|Default|GetCurrentBiomeLength))
        (Game|SpawnActorfromClass "/Game/Blueprints/terrain.Terrain_C" (Math|Transform|MakeTransform (Variables|Default|GetSpawnLocation) "0,90.000000, 0" "1,1,1") "Undefined" 0 0)
        (Variables|Default|SetSpawnLocation (+ (Variables|Default|GetSpawnLocation) "-100.000000, 0, 0"))
        (Variables|Default|SetRowCount (+ (Variables|Default|GetRowCount) 1))))
    (:1
      (for _index_2 (range 0 (Variables|Default|GetCurrentBiomeLength))
        (Game|SpawnActorfromClass "/Game/Blueprints/River.River_C" (Math|Transform|MakeTransform (Variables|Default|GetSpawnLocation) "0,90.000000, 0" "1,1,1") "Undefined" 0 0)
        (Variables|Default|SetSpawnLocation (+ (Variables|Default|GetSpawnLocation) "-100.000000, 0, 0"))
        (Variables|Default|SetRowCount (+ (Variables|Default|GetRowCount) 1))))
    (:2
      (for _index_3 (range 0 (Variables|Default|GetCurrentBiomeLength))
        (Game|SpawnActorfromClass "/Game/Blueprints/Railroad.Railroad_C" (Math|Transform|MakeTransform (Variables|Default|GetSpawnLocation) "0,90.000000, 0" "1,1,1") "Undefined" 0 0)
        (Variables|Default|SetSpawnLocation (+ (Variables|Default|GetSpawnLocation) "-100.000000, 0, 0"))
        (Variables|Default|SetRowCount (+ (Variables|Default|GetRowCount) 1))))
    (:3
      (for _index_4 (range 0 (Variables|Default|GetCurrentBiomeLength))
        (Game|SpawnActorfromClass "/Game/Blueprints/Road.Road_C" (Math|Transform|MakeTransform (Variables|Default|GetSpawnLocation) "0,90.000000, 0" "1,1,1") "Undefined" 0 0)
        (Variables|Default|SetSpawnLocation (+ (Variables|Default|GetSpawnLocation) "-100.000000, 0, 0"))
        (Variables|Default|SetRowCount (+ (Variables|Default|GetRowCount) 1))))))