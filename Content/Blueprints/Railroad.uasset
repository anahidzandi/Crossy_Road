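; Railroad lane actor that periodically sends trains across the track in one direction.
; On BeginPlay it sets its mesh, picks a direction from its X position, then spawns four trains at randomized intervals.
; Each train is a row of separate Train actors: two end pieces around a random number of middle cars.
; Spawning disables the entry-side border's collision, and Train actors are destroyed when they stop overlapping an active border.
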(event OnComponentEndOverlap(RightBorder)
  (params (OverlappedComponent :type Primitive%20Component%20Object%20Reference) (OtherActor :type Actor%20Object%20Reference) (OtherComp :type Primitive%20Component%20Object%20Reference) (OtherBodyIndex :type Integer))
  (bind _astrain (Utilities|Casting|CastToTrain OtherActor))
  (Actor|DestroyActor _astrain))

(event OnComponentEndOverlap(LeftBorder)
  (params (OverlappedComponent :type Primitive%20Component%20Object%20Reference) (OtherActor :type Actor%20Object%20Reference) (OtherComp :type Primitive%20Component%20Object%20Reference) (OtherBodyIndex :type Integer))
  (bind _astrain (Utilities|Casting|CastToTrain OtherActor))
  (Actor|DestroyActor _astrain))

(event EventBeginPlay
  (CallFunction|DetermineDirection)
  (Utilities|FlowControl|Delay (Math|Random|RandomFloatinRange 1.0 5.0))
  (CallFunction|SpawnTrains)
  (Utilities|FlowControl|Delay (Math|Random|RandomFloatinRange 7.0 1e+01))
  (CallFunction|SpawnTrains)
  (Utilities|FlowControl|Delay (Math|Random|RandomFloatinRange 7.0 1e+01))
  (CallFunction|SpawnTrains)
  (Utilities|FlowControl|Delay (Math|Random|RandomFloatinRange 7.0 1e+01))
  (CallFunction|SpawnTrains))

(event Collision|EventActorBeginOverlap
  (params (OtherActor :type Actor%20Object%20Reference)))

(event EventTick
  (params (DeltaSeconds :type Float%20%28single-precision%29)))

(fn ConstructionScript)

(fn DetermineDirection
  (Components|StaticMesh|SetStaticMesh (Variables|Default|GetStaticMesh) "/Game/Meshes/Railroad_Mesh.Railroad_Mesh")
  (Rendering|Material|SetMaterial (Variables|Default|GetStaticMesh) 0 "/Game/Materials/Railroad_Material.Railroad_Material")
  (if (== (Math|Float|%(Float) (.x (Transformation|GetActorLocation)) 2e+02) 0.0)
    (Variables|Default|SetDirectionToRight true)
    (else
      (Variables|Default|SetDirectionToRight false)))
  (Transformation|SetActorLocationAndRotation (+ (Transformation|GetActorLocation) "0, 0,-65.000000") "0,90.000000, 0"))

(fn SpawnTrains
  (Variables|Default|SetLocation (+ (.location (Transformation|GetActorTransform)) "0, 0,20.000000"))
  (if (Variables|Default|GetDirectionToRight)
    (Collision|SetCollisionEnabled (Variables|Default|GetRightBorder) "NoCollision")
    (bind _returnvalue (Game|SpawnActorfromClass "/Game/Blueprints/Train.Train_C" (Math|Transform|MakeTransform (+ (Variables|Default|GetLocation) "0,2000.000000, 0") "0,90.000000, 0" "1,1,1") "Undefined" 0 0))
    (Variables|/Game/Blueprints/Train.Train_C|SetType _returnvalue 0)
    (Variables|/Game/Blueprints/Train.Train_C|SetForwardSpeed _returnvalue -5e+02)
    (Variables|Default|SetLocation (+ (Variables|Default|GetLocation) "0,2000.000000, 0"))
    (for _index (range 0 (Math|Random|RandomIntegerinRange 0 2))
      (bind _returnvalue_2 (Game|SpawnActorfromClass "/Game/Blueprints/Train.Train_C" (Math|Transform|MakeTransform (+ (Variables|Default|GetLocation) "0,465.000000, 0") "0,90.000000, 0" "1,1,1") "Undefined" 0 0))
      (Variables|/Game/Blueprints/Train.Train_C|SetType _returnvalue_2 1)
      (Variables|/Game/Blueprints/Train.Train_C|SetForwardSpeed _returnvalue_2 -5e+02)
      (Variables|Default|SetLocation (+ (Variables|Default|GetLocation) "0,465.000000, 0")))
    (bind _returnvalue_3 (Game|SpawnActorfromClass "/Game/Blueprints/Train.Train_C" (Math|Transform|MakeTransform (+ (Variables|Default|GetLocation) "0,480.000000, 0") "0,90.000000, 0" "1,1,1") "Undefined" 0 0))
    (Variables|/Game/Blueprints/Train.Train_C|SetType _returnvalue_3 2)
    (Variables|/Game/Blueprints/Train.Train_C|SetForwardSpeed _returnvalue_3 -5e+02)
    (else
      (Collision|SetCollisionEnabled (Variables|Default|GetLeftBorder) "NoCollision")
      (bind _returnvalue_4 (Game|SpawnActorfromClass "/Game/Blueprints/Train.Train_C" (Math|Transform|MakeTransform (+ (Variables|Default|GetLocation) "0,-2500.000000, 0") "0,90.000000, 0" "1,1,1") "Undefined" 0 0))
      (Variables|/Game/Blueprints/Train.Train_C|SetType _returnvalue_4 2)
      (Variables|/Game/Blueprints/Train.Train_C|SetForwardSpeed _returnvalue_4 5e+02)
      (Variables|Default|SetLocation (+ (Variables|Default|GetLocation) "0,-2500.000000, 0"))
      (for _index_2 (range 0 (Math|Random|RandomIntegerinRange 0 2))
        (bind _returnvalue_5 (Game|SpawnActorfromClass "/Game/Blueprints/Train.Train_C" (Math|Transform|MakeTransform (+ (Variables|Default|GetLocation) "0,-465.000000, 0") "0,90.000000, 0" "1,1,1") "Undefined" 0 0))
        (Variables|/Game/Blueprints/Train.Train_C|SetType _returnvalue_5 1)
        (Variables|/Game/Blueprints/Train.Train_C|SetForwardSpeed _returnvalue_5 5e+02)
        (Variables|Default|SetLocation (+ (Variables|Default|GetLocation) "0,-465.000000, 0")))
      (bind _returnvalue_6 (Game|SpawnActorfromClass "/Game/Blueprints/Train.Train_C" (Math|Transform|MakeTransform (+ (Variables|Default|GetLocation) "0,-480.000000, 0") "0,90.000000, 0" "1,1,1") "Undefined" 0 0))
      (Variables|/Game/Blueprints/Train.Train_C|SetType _returnvalue_6 0)
      (Variables|/Game/Blueprints/Train.Train_C|SetForwardSpeed _returnvalue_6 5e+02))))