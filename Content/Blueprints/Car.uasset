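; Car actor that drives along the world Y axis and kills any chicken it hits.
; On BeginPlay, Randomize picks one of six car variants, using a single random index to set matching mesh, material and collision box size.
; Tick offsets the actor by ForwardSpeed scaled by delta time.
; Box overlap with a Chicken_BP sets that chicken's IsDead flag.
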(event OnComponentBeginOverlap(Box)
  (params (OverlappedComponent :type Primitive%20Component%20Object%20Reference) (OtherActor :type Actor%20Object%20Reference) (OtherComp :type Primitive%20Component%20Object%20Reference) (OtherBodyIndex :type Integer) (bFromSweep :type Boolean) (SweepResult :type Hit%20Result%20Structure%20%28by%20ref%29))
  (bind _aschicken_bp (Utilities|Casting|CastToChicken_BP OtherActor))
  (Variables|/Game/Blueprints/Chicken_BP.Chicken_BP_C|SetIsDead _aschicken_bp true))

(event EventBeginPlay
  (CallFunction|Randomize))

(event Collision|EventActorBeginOverlap
  (params (OtherActor :type Actor%20Object%20Reference)))

(event EventTick
  (params (DeltaSeconds :type Float%20%28single-precision%29))
  (Transformation|AddActorWorldOffset (Math|Vector|MakeVector 0.0 (* DeltaSeconds (Variables|Default|GetForwardSpeed)) 0.0)))

(fn ConstructionScript)

(fn Randomize
  (bind _output_get (LocalVariables|SetRandomInt (Math|Random|RandomIntegerinRange 0 5)))
  (Components|StaticMesh|SetStaticMesh (Variables|Default|GetStaticMesh) (Utilities|Select :Index _output_get :Option%200 "/Game/Meshes/Car_Blue_Mesh.Car_Blue_Mesh" :Option%201 "/Game/Meshes/Car_Green_Mesh.Car_Green_Mesh" :Option%202 "/Game/Meshes/Car_Police_Mesh.Car_Police_Mesh" :Option%203 "/Game/Meshes/Car_Purple_Mesh.Car_Purple_Mesh" :Option%204 "/Game/Meshes/Car_Red_Mesh.Car_Red_Mesh" :Option%205 "/Game/Meshes/Car_Taxi_Mesh.Car_Taxi_Mesh"))
  (Rendering|Material|SetMaterial (Variables|Default|GetStaticMesh) 0 (Utilities|Select :Index _output_get :Option%200 "/Game/Materials/Car_Blue_Material.Car_Blue_Material" :Option%201 "/Game/Materials/Car_Green_Material.Car_Green_Material" :Option%202 "/Game/Materials/Car_Police_Material.Car_Police_Material" :Option%203 "/Game/Materials/Car_Purple_Material.Car_Purple_Material" :Option%204 "/Game/Materials/Car_Red_Material.Car_Red_Material" :Option%205 "/Game/Materials/Car_Taxi_Material.Car_Taxi_Material"))
  (Components|Box|SetBoxExtent (Variables|Default|GetBox) (Utilities|Select :Index _output_get :Option%200 "43.000000,67.000000,35.000000" :Option%201 "43.000000,103.000000,35.000000" :Option%202 "43.000000,91.000000,35.000000" :Option%203 "43.000000,91.000000,35.000000" :Option%204 "43.000000,91.000000,35.000000" :Option%205 "43.000000,91.000000,35.000000") true))